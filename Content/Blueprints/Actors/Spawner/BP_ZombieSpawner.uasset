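; Spawner actor that periodically creates BP_Zombie enemies at its own transform.
; A looping timer started on BeginPlay fires every SpawnInterval, adjusting placement to avoid collisions or skipping the spawn if none fits.
; Each successful spawn gets a default controller and increments a counter, stopping the timer at MaxSpawnCount, where zero means unlimited.
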(event `self.ReceiveBeginPlay`
  (bind _returnvalue (`KismetSystemLibrary.K2_SetTimerDelegate` (delegate `SpawnZombie`) (`self.SpawnInterval`) true)))

(event `SpawnZombie`
  (bind _returnvalue (`|SpawnActorFromClass` "/Game/Blueprints/Characters/Zombie/BP_Zombie.BP_Zombie_C" (`self.GetTransform`) "AdjustIfPossibleButDontSpawnIfColliding" "OverrideRootScale" null null))
  (`/Engine/EditorBlueprintResources/StandardMacros.IsValid` _returnvalue
    (:`Is Valid`
      (`Pawn.SpawnDefaultController` _returnvalue)
      (`/Engine/EditorBlueprintResources/StandardMacros.IncrementInt` (`self.CurrentSpawnCount`)
        (:`  `
          (if (and (!= (`self.MaxSpawnCount`) 0) (>= (`self.CurrentSpawnCount`) (`self.MaxSpawnCount`)))
            (`KismetSystemLibrary.K2_ClearAndInvalidateTimerHandle` (stale `self.ReceiveBeginPlay` _returnvalue))))))))

(fn `UserConstructionScript`)